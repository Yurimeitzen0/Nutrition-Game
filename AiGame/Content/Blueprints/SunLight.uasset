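; SunLight is a timed magic-circle area effect that periodically sends DoFireDamage with a SunLightRestore value to actors inside it, using heal-themed materials.
; A capsule tracks overlapping IsUsable actors in the Character array, which a looping timer walks to send the interface message.
; On BeginPlay, dynamic materials are created for the circle's layers, and the MagicTime timeline drives their Vis parameter before deactivating the effect and destroying the actor.
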(event OnComponentBeginOverlap(Capsule)
  (params (OverlappedComponent :type Primitive%20Component%20Object%20Reference) (OtherActor :type Actor%20Object%20Reference) (OtherComp :type Primitive%20Component%20Object%20Reference) (OtherBodyIndex :type Integer) (bFromSweep :type Boolean) (SweepResult :type Hit%20Result%20Structure%20%28by%20ref%29))
  (if (Utilities|DoesObjectImplementInterface OtherActor "/Game/Interfaces/IsUsable.IsUsable_C")
    (Utilities|Array|AddUnique (Variables|Default|GetCharacter) OtherActor)))

(event OnComponentEndOverlap(Capsule)
  (params (OverlappedComponent :type Primitive%20Component%20Object%20Reference) (OtherActor :type Actor%20Object%20Reference) (OtherComp :type Primitive%20Component%20Object%20Reference) (OtherBodyIndex :type Integer))
  (if (Utilities|DoesObjectImplementInterface OtherActor "/Game/Interfaces/IsUsable.IsUsable_C")
    (Utilities|Array|RemoveItem (Variables|Default|GetCharacter) OtherActor)))

(event Custom|DamageInsideArea
  (if (== (Utilities|Array|Length (Variables|Default|GetCharacter)) 0)
    (Development|PrintString "False")
    (else
      (for _array_element (Variables|Default|GetCharacter)
        (if (Collision|IsOverlappingActor _array_element :!class /Script/Engine.Actor)
          (if (Utilities|DoesObjectImplementInterface _array_element "/Game/Interfaces/IsUsable.IsUsable_C")
            (Class|IsUsable|DoFireDamage(Message) _array_element (Variables|Default|GetSunLightRestore))))))))

(event Custom|test
  ;[1 1 1] Like This
  (Utilities|Time|SetTimerbyEvent (delegate Custom|test) 0.0))

(event EventBeginPlay
  (bind (_magicring _symbol _magicdot _beam _magiccircle) (Utilities|CreateDynamicMagicMaterial))
  (Utilities|Time|SetTimerbyEvent (delegate Custom|DamageInsideArea) 2.0 true)
  (bind _fadeamount (Timeline|MagicTime PlayFromStart)
    (:Update
      (Utilities|FadeMaterial _magicring _symbol _magicdot _beam _magiccircle _fadeamount))
    (:Finished
      (Components|Activation|Deactivate (Variables|Default|GetMagic_Circle))
      (Actor|DestroyActor))))

(fn ConstructionScript)