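; A Sonic-style jump pad actor that springs the player character into the air when it overlaps the pad.
; On begin overlap, an exact class check for AIS_Character gates a LaunchCharacter call along the Pad component's up vector, scaled by SpringPower.
; The launch overrides both XY and Z velocity, so the pad's rotation sets the direction.
; It also plays a 2D spring sound and prints the up vector for debugging.
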(event EventBeginPlay)

(event Collision|EventActorBeginOverlap
  (params (OtherActor :type Actor%20Object%20Reference))
  (bind _pad (Variables|Default|GetPad))
  (bind _returnvalue (Math|Vector|GetUpVector _pad))
  (if (== (Utilities|GetClass OtherActor) "/Game/Blueprints/AI/AIS_Character.AIS_Character_C")
    (bind _ascharacter (Utilities|Casting|CastToCharacter OtherActor))
    (Character|LaunchCharacter _ascharacter (* _returnvalue (Variables|Default|GetSpringPower)) true true)
    (Audio|PlaySound2D "/Game/Blueprints/Audio/sonic-spring.sonic-spring" 1.0 1.0 0.0 0 0)
    (Development|PrintString (Utilities|String|ToString(Vector) _returnvalue))))

(event EventTick
  (params (DeltaSeconds :type Float%20%28single-precision%29)))

(fn ConstructionScript)