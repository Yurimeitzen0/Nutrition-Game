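; Food item that AI characters perceive by sight and consume to restore stats and add game score.
; UseItem adds StatRestore to each AiStatArray entry, clamped to its limits, applies damage if the first value is non-positive, then destroys itself shortly after.
; The SetAbsorptionBlocker macro intercepts two stats when their blocker stat is low, overwriting them with the blocker's entry.
; BeginPlay registers the sight stimulus and gives the mesh random spin.
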(event Custom|Post%20Use
  (Utilities|FlowControl|Delay 0.1)
  (Actor|DestroyActor))

(event EventBeginPlay
  ;[1 1 1] Optional?
  (Class|AIPerceptionSystem|RegisterPerceptionStimuliSource "/Script/AIModule.AISense_Sight" self)
  (Class|PrimitiveComponent|SetPhysicsAngularVelocityinDegrees (Variables|Default|GetFoodMesh) (* (Math|Random|RandomUnitVector) 1e+02) false "None"))

(event EventUseItem
  (params (AI%20Character :type AIS%20Character%20Object%20Reference))
  (bind _aistatarray (Variables|/Game/Blueprints/AI/AIS_Character.AIS_Character_C|GetAiStatArray AI%20Character))
  (bind _statrestore (Variables|Default|GetStatRestore))
  (bind _output (Utilities|Array|Get(acopy) _statrestore))
  (for _index (range 0 (Utilities|Array|LastIndex _aistatarray))
    (bind (_itemsarray _currentindex _item) (Utilities|SetAbsorptionBlocker _aistatarray 7 _index 3)
      (:True
        (Utilities|Array|SetArrayElem _itemsarray _currentindex _item))
      (:False
        (bind (_itemsarray_2 _currentindex_2 _item_2) (Utilities|SetAbsorptionBlocker _aistatarray 6 _index 4)
          (:True
            (Utilities|Array|SetArrayElem _itemsarray_2 _currentindex_2 _item_2))
          (:False
            (Utilities|Array|SetArrayElem _aistatarray _index (Utilities|Struct|MakeFoodStruct (Math|Float|Clamp(Float) (+ (Utilities|Array|Get(acopy) (Variables|Default|GetStatRestore) _index) (.CurrentStatValue (Utilities|Struct|BreakFoodStruct (Utilities|Array|Get(acopy) _aistatarray _index)))) (.MinStat (Utilities|Struct|BreakFoodStruct (Utilities|Array|Get(acopy) _aistatarray _index))) (.MaxStat (Utilities|Struct|BreakFoodStruct (Utilities|Array|Get(acopy) _aistatarray _index)))) (.MinStat (Utilities|Struct|BreakFoodStruct (Utilities|Array|Get(acopy) _aistatarray _index))) (.MaxStat (Utilities|Struct|BreakFoodStruct (Utilities|Array|Get(acopy) _aistatarray _index))) (.StatDesirability (Utilities|Struct|BreakFoodStruct (Utilities|Array|Get(acopy) _aistatarray _index))) (.StatDecayRate (Utilities|Struct|BreakFoodStruct (Utilities|Array|Get(acopy) _aistatarray _index))) (.StatBehaviors (Utilities|Struct|BreakFoodStruct (Utilities|Array|Get(acopy) _aistatarray _index))) false (> (Utilities|Array|Get(acopy) (Variables|Default|GetStatRestore) _index) 0.0))))))))
  (if (<= _output 0.0)
    (Game|Damage|ApplyDamage AI%20Character (Math|Float|Absolute(Float) _output) 0 self))
  (bind _asais_game_mode (Utilities|Casting|CastToAIS_GameMode (Game|GetGameMode)))
  (Variables|/Game/Blueprints/AIS_GameMode.AIS_GameMode_C|SetScore _asais_game_mode (+ (Variables|/Game/Blueprints/AIS_GameMode.AIS_GameMode_C|GetScore _asais_game_mode) 5))
  (CallFunction|PostUse))

(fn ConstructionScript)