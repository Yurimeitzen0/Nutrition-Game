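; UpperFloorR is a moving floor actor that shuttles its static mesh between the Pos1 and Pos2 markers in an endless loop.
; On BeginPlay it places Default at the mesh's location and starts the Infinite timeline.
; When the timeline finishes, chained eased MoveComponentTo calls and pauses run Pos1, Pos2, Pos2, Pos1, then restart the timeline.
; The markers' world transforms feed the relative-space move targets.
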(event EventBeginPlay
  (bind _pos2 (Variables|Default|GetPos2))
  (bind _pos2_2 (Variables|Default|GetPos2))
  (bind _pos1 (Variables|Default|GetPos1))
  (bind _pos1_2 (Variables|Default|GetPos1))
  (Transformation|SetWorldLocation (Variables|Default|GetDefault) (Transformation|GetWorldLocation (Variables|Debug|GetStaticMeshComponent)) false false)
  (Timeline|infinite Play
    (:Finished
      (Components|MoveComponentTo (Variables|Debug|GetStaticMeshComponent) (Transformation|GetWorldLocation _pos1) (Transformation|GetWorldRotation _pos1) true true 6.0 false)
      (Utilities|FlowControl|Delay 1.0)
      (Components|MoveComponentTo (Variables|Debug|GetStaticMeshComponent) (Transformation|GetWorldLocation _pos2) (Transformation|GetWorldRotation _pos2) true true 6.0 false)
      (Utilities|FlowControl|Delay 1.0)
      (Components|MoveComponentTo (Variables|Debug|GetStaticMeshComponent) (Transformation|GetWorldLocation _pos2_2) (Transformation|GetWorldRotation _pos2_2) true true 6.0 false)
      (Utilities|FlowControl|Delay 1.0)
      (Components|MoveComponentTo (Variables|Debug|GetStaticMeshComponent) (Transformation|GetWorldLocation _pos1_2) (Transformation|GetWorldRotation _pos1_2) true true 6.0 false)
      (Utilities|FlowControl|Delay 1.0)
      (Timeline|infinite PlayFromStart))))

(fn ConstructionScript)