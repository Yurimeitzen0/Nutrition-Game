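; UpperFloor is an actor whose static mesh moves back and forth endlessly between two marker components, Pos1 and Pos2.
; On BeginPlay it stores the mesh's start location in the Default component, then starts the Infinite timeline.
; When the timeline finishes, a chain of eased MoveComponentTo calls and short delays runs, then restarts the timeline to loop.
; The markers' world locations serve as relative move targets, and repeated targets lengthen the stops.
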(event EventBeginPlay
  (Transformation|SetWorldLocation (Variables|Default|GetDefault) (Transformation|GetWorldLocation (Variables|Debug|GetStaticMeshComponent)) false false)
  (Timeline|infinite Play
    (:Finished
      (Components|MoveComponentTo (Variables|Debug|GetStaticMeshComponent) (Transformation|GetWorldLocation (Variables|Default|GetPos1)) "0, 0, 0" true true 6.0 false)
      (Utilities|FlowControl|Delay 1.0)
      (Components|MoveComponentTo (Variables|Debug|GetStaticMeshComponent) (Transformation|GetWorldLocation (Variables|Default|GetPos2)) "0, 0, 0" true true 6.0 false)
      (Utilities|FlowControl|Delay 1.0)
      (Components|MoveComponentTo (Variables|Debug|GetStaticMeshComponent) (Transformation|GetWorldLocation (Variables|Default|GetPos2)) "0, 0, 0" true true 6.0 false)
      (Utilities|FlowControl|Delay 1.0)
      (Components|MoveComponentTo (Variables|Debug|GetStaticMeshComponent) (Transformation|GetWorldLocation (Variables|Default|GetPos1)) "0, 0, 0" true true 6.0 false)
      (Utilities|FlowControl|Delay 1.0)
      (Timeline|infinite PlayFromStart))))

(fn ConstructionScript)