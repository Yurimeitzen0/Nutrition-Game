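; Tree is an objective actor that the player character checks off by touching it.
; On BeginPlay it casts the game mode to AIS_GameMode, caches it and increments its Objective counter, so each placed tree adds to the total.
; The first overlap by an actor of exactly the AIS_Character class sets Checked and decrements that counter, so each tree counts only once.
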(event EventBeginPlay
  (bind _asais_game_mode (Utilities|Casting|CastToAIS_GameMode (Game|GetGameMode)))
  (bind _output_get (Variables|Default|SetGameMode _asais_game_mode))
  (bind _result (Math|Integer|IncrementInt (Variables|/Game/Blueprints/AIS_GameMode.AIS_GameMode_C|GetObjective _output_get))
    (:%20%20
      (Variables|/Game/Blueprints/AIS_GameMode.AIS_GameMode_C|SetObjective _output_get _result))))

(event Collision|EventActorBeginOverlap
  (params (OtherActor :type Actor%20Object%20Reference))
  (bind _gamemode (Variables|Default|GetGameMode))
  (if (and (== (Utilities|GetClass OtherActor) "/Game/Blueprints/AI/AIS_Character.AIS_Character_C") (Math|Boolean|Equal(Boolean) (Variables|Default|GetChecked) false))
    (Variables|Default|SetChecked true)
    (bind _result (Math|Integer|DecrementInt (Variables|/Game/Blueprints/AIS_GameMode.AIS_GameMode_C|GetObjective _gamemode))
      (:%20%20
        (Variables|/Game/Blueprints/AIS_GameMode.AIS_GameMode_C|SetObjective _gamemode _result)))))

(event EventTick
  (params (DeltaSeconds :type Float%20%28single-precision%29)))

(fn ConstructionScript)