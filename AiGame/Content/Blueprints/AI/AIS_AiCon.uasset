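; AIS_AiCon is an AI controller that starts the AIS_BT behavior tree on BeginPlay.
; Its TasktoController event relays a montage index to the controlled pawn through ControllerToCharacterMessage, bridging a caller and the character.
; The AIPerception update events are empty, and the debug print nodes for perceived actors are left disconnected.
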(event OnPerceptionUpdated(AIPerception)
  (params (UpdatedActors :type Array%20of%20Actor%20Object%20References)))

(event OnTargetPerceptionUpdated(AIPerception)
  (params (Actor :type Actor%20Object%20Reference) (Stimulus :type AI%20Stimulus%20Structure)))

(event EventBeginPlay
  (AI|RunBehaviorTree "/Game/Blueprints/AI/AIS_BT.AIS_BT"))

(event EventTasktoController
  (params (MontageIndex :type Integer))
  (Class|AIAnimation|ControllertoCharacter(Message) (Pawn|GetControlledPawn) MontageIndex))

(fn ConstructionScript)