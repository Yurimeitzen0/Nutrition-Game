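; AI character with survival stats that decay over time and visibly affect its body.
; BeginPlay loads stats from a DataTable and starts a looping decay timer; low stats deal damage to the health stat, destroying the character at zero.
; Tick maps stats to dynamic-material symptoms (eyes, head, tummy, skin), mesh width, partial physical-animation ragdoll and walk speed.
; Events also handle sunlight exposure, interface-based item use, dialogue callouts and AnimBP montage messages.
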(event Custom|Starve
  (for (_ _array_index) (Variables|Default|GetAiStatArray)
    (if (!= _array_index 1)
      (CallFunction|StatTickDown _array_index) ; Ticks Hunger(stat 2)
    )))

(event Custom|DialogCallout
  (params (ThingToTalkAbout :type Actor%20Object%20Reference))
  (bind _mesh (Variables|Character|GetMesh))
  ;[1 1 1] Dialogue Handler For Identifying object
  (Class|GameplayStatics|SpawnDialogueAttached "/Game/Blueprints/Audio/IFound_Gender.IFound_Gender" (Utilities|Struct|MakeDialogueContext (Utilities|Array|Get(acopy) (Variables|/Game/Blueprints/DialogComponent.DialogComponent_C|GetDialogContext (Variables|Default|GetDialogComponent))) (Variables|/Game/Blueprints/DialogComponent.DialogComponent_C|GetDialogContext (Actor|GetComponentbyClass ThingToTalkAbout "/Game/Blueprints/DialogComponent.DialogComponent_C"))) _mesh "head" (Transformation|GetWorldLocation _mesh) "0, 0, 0" "KeepRelativeOffset" false 1.0 1.0 0.0 0))

(event EventBeginPlay
  (Utilities|Time|SetTimerbyEvent (delegate Custom|Starve) (Variables|Default|GetStatTickRate) true) ; Custom Tick for stamina consumption
  ;[1 1 1] Sets the current pawn for stats update on widget
  (Variables|/Game/UI/StatBlock.StatBlock_C|SetOwningPawn (.AsStat%20Block (Utilities|Casting|CastToStatBlock (UserInterface|GetUserWidgetObject (Variables|Default|GetHUD)))) self)
  (bind _asais_game_state (Utilities|Casting|CastToAIS_GameState (Game|GetGameState))
    (:then
      (bind _output_get (Variables|Default|SetStoredGameState _asais_game_state))
      (bind _outrownames (DataTable|GetDataTableRowNames "/Game/Blueprints/AI/DataTable/StatTable.StatTable"))
      (bind _output_get_2 (Variables|/Game/Blueprints/AIS_GameState.AIS_GameState_C|SetStatNames _output_get _outrownames))
      (bind _output_get_3 (Variables|Default|SetStatName _output_get_2))
      (for _array_element _output_get_3
        (bind _returnvalue (Utilities|GetDataTableRow "/Game/Blueprints/AI/DataTable/StatTable.StatTable" _array_element)
          (:then
            (Utilities|Array|Add (Variables|Default|GetAiStatArray) _returnvalue)))))
    (:CastFailed
      (Development|PrintString "somthing something"))))

(event EventTick
  (params (DeltaSeconds :type Float%20%28single-precision%29))
  (bind _physicalanimationdata (Utilities|Struct|MakePhysicalAnimationData true 1e+02 5e+01 1e+02 5e+01))
  (bind _mesh (Variables|Character|GetMesh))
  (bind _physicalanimation (Variables|Default|GetPhysicalAnimation))
  (bind _aistatarray (Variables|Default|GetAiStatArray))
  (bind _bones (Variables|Default|GetBones))
  (bind _bones_2 (Variables|Default|GetBones))
  (bind _physicalanimation_2 (Variables|Default|GetPhysicalAnimation))
  (bind _charactermovement (Variables|Character|GetCharacterMovement))
  (bind _aistatarray_2 (Variables|Default|GetAiStatArray))
  (bind _mesh_2 (Variables|Character|GetMesh))
  (bind _output (Utilities|Array|Get(acopy) _aistatarray 11))
  (bind _currentstatvalue (Utilities|Struct|BreakFoodStruct _output))
  (bind _returnvalue (|(3.500000-(1/((A+0.100000)/100))) _currentstatvalue))
  (bind _returnvalue_2 (Math|Float|Clamp(Float) _returnvalue 0.57))
  (Utilities|FlowControl|Sequence
    (:then_0
      (Transformation|SetWorldLocation (Variables|Default|GetEyeSockets) (Transformation|GetSocketLocation _mesh "Eyes") false false)
      (Rendering|Material|SetScalarParameterValue (Variables|Default|GetI_Reye) "Opacity" (|((1/(A/100))-2) (.CurrentStatValue (Utilities|Struct|BreakFoodStruct (Utilities|Array|Get(acopy) _aistatarray 5)))) :!class /Script/Engine.MaterialInstanceDynamic))
    (:then_1
      (Transformation|SetWorldLocation (Variables|Default|GetHeadAche) (Transformation|GetSocketLocation _mesh "headSocket") false false)
      (Rendering|Material|SetScalarParameterValue (Variables|Default|GetI_Head) "Opacity" (|((1/(A/100))-2) (.CurrentStatValue (Utilities|Struct|BreakFoodStruct (Utilities|Array|Get(acopy) _aistatarray 9)))) :!class /Script/Engine.MaterialInstanceDynamic))
    (:then_2
      (Transformation|SetWorldLocation (Variables|Default|GetTummy) (Transformation|GetSocketLocation _mesh "Tummy") false false)
      (Rendering|Material|SetScalarParameterValue (Variables|Default|GetI_Tummy) "Opacity" (|((1/(A/100))-2) (.CurrentStatValue (Utilities|Struct|BreakFoodStruct (Utilities|Array|Get(acopy) _aistatarray 8)))) :!class /Script/Engine.MaterialInstanceDynamic))
    (:then_3
      (Transformation|SetWorldTransform _mesh_2 (Math|Transform|MakeTransform (Transformation|GetWorldLocation _mesh_2) (Transformation|GetWorldRotation _mesh_2) (Math|Vector|MakeVector _returnvalue_2 _returnvalue_2 1.0)) false false))
    (:then_4
      (if (<= (.CurrentStatValue (Utilities|Struct|BreakFoodStruct (Utilities|Array|Get(acopy) _aistatarray_2 3))) 5e+01)
        (Class|PhysicalAnimationComponent|SetSkeletalMeshComponent _physicalanimation_2 (Variables|Character|GetMesh))
        (Class|PhysicalAnimationComponent|ApplyPhysicalAnimationSettingsBelow _physicalanimation_2 _bones_2 _physicalanimationdata false)
        (Class|SkeletalMeshComponent|SetAllBodiesBelowSimulatePhysics (Variables|Character|GetMesh) _bones_2 true false)
        (else
          (Class|PhysicalAnimationComponent|SetSkeletalMeshComponent _physicalanimation (Variables|Character|GetMesh))
          (Class|PhysicalAnimationComponent|ApplyPhysicalAnimationSettingsBelow _physicalanimation _bones _physicalanimationdata false)
          (Class|SkeletalMeshComponent|SetAllBodiesBelowSimulatePhysics (Variables|Character|GetMesh) _bones false false))))
    (:then_5
      (Utilities|FlowControl|Sequence
        (:then_0
          (Rendering|Material|SetScalarParameterValue (Variables|Default|GetI_Skin) "Skin" (Math|Float|Clamp(Float) (|((1/(A/100))-1.500000) (.CurrentStatValue (Utilities|Struct|BreakFoodStruct (Utilities|Array|Get(acopy) _aistatarray_2 4))))) :!class /Script/Engine.MaterialInstanceDynamic))
        (:then_1
          (if (not (or (<= (.CurrentStatValue (Utilities|Struct|BreakFoodStruct (Utilities|Array|Get(acopy) (Variables|Default|GetAiStatArray) 2))) 3e+01) (<= (.CurrentStatValue (Utilities|Struct|BreakFoodStruct (Utilities|Array|Get(acopy) (Variables|Default|GetAiStatArray) 10))) 8e+01)))
            (Variables|/Script/Engine.CharacterMovementComponent|SetMaxWalkSpeed _charactermovement 4.5e+02)
            (else
              (Variables|/Script/Engine.CharacterMovementComponent|SetMaxWalkSpeed _charactermovement 1.5e+02))))))))

(event EventAiUseItem
  (params (ItemToUse :type Actor%20Object%20Reference))
  ;[1 1 1] Using item with the desired interface
  (if (Utilities|DoesObjectImplementInterface ItemToUse "/Game/Interfaces/IsUsable.IsUsable_C")
    (Class|IsUsable|UseItem(Message) ItemToUse self)
    (else
      (Development|PrintString "Unusable Item"))))

(event Game|Damage|EventAnyDamage
  (params (Damage :type Float%20%28single-precision%29) (DamageType :type Damage%20Type%20Object%20Reference) (InstigatedBy :type Controller%20Object%20Reference) (DamageCauser :type Actor%20Object%20Reference))
  (bind _aistatarray (Variables|Default|GetAiStatArray))
  (bind _output (Utilities|Array|Get(acopy) _aistatarray 1))
  (bind (_currentstatvalue _minstat _maxstat _statdesirability _statdecayrate _statbehaviors) (Utilities|Struct|BreakFoodStruct _output))
  (bind _returnvalue (- _currentstatvalue Damage))
  (bind _returnvalue_2 (Math|Float|Clamp(Float) _returnvalue _minstat _maxstat))
  ;[1 1 1] Handles damage logic
  (Development|PrintString "I'm Starving")
  (Utilities|Array|SetArrayElem (Variables|Default|GetAiStatArray) 1 (Utilities|Struct|MakeFoodStruct _returnvalue_2 _minstat _maxstat _statdesirability _statdecayrate _statbehaviors))
  (if (<= _returnvalue_2 0.0)
    (Pawn|UnPossess (Pawn|GetController))
    (Actor|DestroyActor)))

(event EventDoFireDamage
  (params (AiCharacter :type AIS%20Character%20Object%20Reference) (Sunlight :type Float%20%28single-precision%29))
  (bind _aistatarray (Variables|Default|GetAiStatArray))
  (bind _output (Utilities|Array|Get(acopy) _aistatarray 7))
  (bind (_currentstatvalue _minstat _maxstat _statdesirability _statdecayrate _statbehaviors _nutrientdebuff) (Utilities|Struct|BreakFoodStruct _output))
  (Utilities|Array|SetArrayElem _aistatarray 7 (Utilities|Struct|MakeFoodStruct (Math|Float|Clamp(Float) (+ Sunlight _currentstatvalue) 0.0 1e+02) _minstat _maxstat _statdesirability _statdecayrate _statbehaviors _nutrientdebuff)))

(event EventControllertoCharacter
  (params (MontageIndex :type Integer))
  (Class|AIAnimation|CharactertoAnimBP(Message) (Components|SkeletalMesh|GetAnimInstance (Variables|Character|GetMesh)) MontageIndex))

(fn ConstructionScript
  (Utilities|FlowControl|Sequence
    (:then_0
      (bind _returnvalue (Rendering|Material|CreateDynamicMaterialInstance (Variables|Default|GetL_eye) 0 "/Game/Blueprints/Assets/M_instances/M_Eye_Inst.M_Eye_Inst" "R_eye" :!class /Script/Engine.PrimitiveComponent))
      (bind _output_get (Variables|Default|SetI_Leye _returnvalue)))
    (:then_1
      (bind _returnvalue_2 (Rendering|Material|CreateDynamicMaterialInstance (Variables|Default|GetR_eye) 0 "/Game/Blueprints/Assets/M_instances/M_Eye_Inst.M_Eye_Inst" "L_eye" :!class /Script/Engine.PrimitiveComponent))
      (bind _output_get_2 (Variables|Default|SetI_Reye _returnvalue_2))
      (Rendering|Material|SetScalarParameterValue _output_get "Opacity" 0.0 :!class /Script/Engine.MaterialInstanceDynamic))
    (:then_2
      (bind _returnvalue_3 (Rendering|Material|CreateDynamicMaterialInstance (Variables|Default|GetHeadAche) 0 "/Game/Blueprints/Assets/M_instances/M_Headache_Inst.M_Headache_Inst" "None" :!class /Script/Engine.PrimitiveComponent))
      (bind _output_get_3 (Variables|Default|SetI_Head _returnvalue_3))
      (Rendering|Material|SetScalarParameterValue _output_get_3 "Opacity" 0.0 :!class /Script/Engine.MaterialInstanceDynamic))
    (:then_3
      (bind _returnvalue_4 (Rendering|Material|CreateDynamicMaterialInstance (Variables|Default|GetTummy) 0 "/Game/Blueprints/Assets/M_instances/M_TummyAche_Inst_Inst.M_TummyAche_Inst_Inst" "None" :!class /Script/Engine.PrimitiveComponent))
      (bind _output_get_4 (Variables|Default|SetI_Tummy _returnvalue_4))
      (Rendering|Material|SetScalarParameterValue _output_get_4 "Opacity" 0.0 :!class /Script/Engine.MaterialInstanceDynamic))
    (:then_4
      (bind _returnvalue_5 (Rendering|Material|CreateDynamicMaterialInstance (Variables|Character|GetMesh) 0 "/Game/Mannequin/Character/Materials/M_UE4Man_Body.M_UE4Man_Body" "None" :!class /Script/Engine.PrimitiveComponent))
      (bind _output_get_5 (Variables|Default|SetI_Skin _returnvalue_5))
      (Rendering|Material|SetScalarParameterValue _output_get_5 "Skin" 0.0 :!class /Script/Engine.MaterialInstanceDynamic))))

(fn StatTickDown
  (params (StatToTick :type Integer))
  (bind _self self)
  (bind _stattickrate (Variables|Default|GetStatTickRate))
  (bind _aistatarray (Variables|Default|GetAiStatArray))
  (bind _output (Utilities|Array|Get(acopy) _aistatarray StatToTick))
  (bind (_currentstatvalue _minstat _maxstat _statdesirability _statdecayrate _statbehaviors) (Utilities|Struct|BreakFoodStruct _output))
  (bind _returnvalue (* _statdecayrate _stattickrate))
  (bind _returnvalue_2 (- _currentstatvalue _returnvalue))
  (bind _returnvalue_3 (<= _returnvalue_2 3e+01))
  (bind _returnvalue_4 (Math|Float|Clamp(Float) _returnvalue_2 _minstat _maxstat))
  (bind _foodstruct (Utilities|Struct|MakeFoodStruct _returnvalue_4 _minstat _maxstat _statdesirability _statdecayrate _statbehaviors _returnvalue_3))
  (Utilities|Array|SetArrayElem (Variables|Default|GetAiStatArray) StatToTick _foodstruct)
  (if (.NutrientDebuff (Utilities|Struct|BreakFoodStruct _foodstruct))
    (Game|Damage|ApplyDamage _self 1.0 0 _self)))