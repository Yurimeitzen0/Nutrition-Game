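; Player controller that moves the camera pawn, selects IsUsable actors and lets the player drop food or sunlight into the world.
; Left-click traces under the cursor to select an actor and fill the StatBlock HUD; a short right-click deselects, while holding it rotates the camera through a Tick-driven gate.
; Hotkeys spawn items at the cursor, some randomized within a food group, each deducting GameMode score.
; Pause functions toggle the menu and score widget.
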(event Custom|LeftClickAction)

(event Custom|RightClickAction
  (bind _storedpawn (Variables|Default|GetStoredPawn))
  (bind _hud (Variables|/Game/Blueprints/AIS_PlayerPawn.AIS_PlayerPawn_C|GetHUD _storedpawn))
  (bind _returnvalue (UserInterface|GetUserWidgetObject _hud))
  (Utilities|IsValid (Variables|Default|GetSelectedThing)
    (:Is%20Valid
      (Class|IsUsable|Deselected(Message) (Variables|Default|GetSelectedThing))
      (Variables|Default|SetSelectedThing 0)
      (Widget|SetVisibility _returnvalue "Hidden")
      (bind _asstat_block (Utilities|Casting|CastToStatBlock _returnvalue))
      (Default|ClearPawn _asstat_block))))

(event EventBeginPlay
  (bind _asais_game_mode (Utilities|Casting|CastToAIS_GameMode (Game|GetGameMode)))
  (Variables|Default|SetGameMode _asais_game_mode))

(event EventTick
  (params (DeltaSeconds :type Float%20%28single-precision%29))
  (bind (_locationx _locationy) (Game|Player|GetMousePosition))
  (bind (_locationx_2 _locationy_2) (Game|Player|GetMousePosition))
  (bind _returnvalue (Pawn|GetControlRotation :!class /Script/Engine.Controller))
  (bind _storedpawn (Variables|Default|GetStoredPawn))
  (bind (_roll _pitch _yaw) (Math|Rotator|BreakRotator _returnvalue))
  (bind _springarm (Variables|/Game/Blueprints/AIS_PlayerPawn.AIS_PlayerPawn_C|GetSpringArm _storedpawn))
  (bind _returnvalue_2 (Transformation|GetWorldRotation _springarm))
  (bind (_roll_2 _pitch_2 _yaw_2) (Math|Rotator|BreakRotator _returnvalue_2))
  (Utilities|FlowControl|Sequence
    (:then_0
      (Utilities|FlowControl|Gate true
        (:Exit
          (if (Variables|Default|GetbLeftClick)
            (if (>= (Variables|Default|GetLeftClickHoldCounter) 0.06)
              (Variables|Default|SetbLeftClick false)
              (else
                (Variables|Default|SetLeftClickHoldCounter (+ DeltaSeconds (Variables|Default|GetLeftClickHoldCounter)))))))))
    (:then_1
      (Utilities|FlowControl|Gate true
        (:Exit
          (if (Variables|Default|GetbRightClick)
            (if (>= (Variables|Default|GetRightClickHoldCounter) 0.06)
              (Variables|Default|SetbRightClick false)
              (else
                (Variables|Default|SetRightClickHoldCounter (+ DeltaSeconds (Variables|Default|GetRightClickHoldCounter)))))
            (else
              (Pawn|SetControlRotation (Math|Rotator|MakeRotator 0.0 0.0 (+ (Class|Actor|GetInputAxisKeyValue) (.Yaw (Math|Rotator|BreakRotator (Pawn|GetControlRotation :!class /Script/Engine.Controller))))))
              (Transformation|SetWorldRotation _springarm (Math|Rotator|MakeRotator 0.0 (+ (Class|Actor|GetInputAxisKeyValue) _pitch_2) (+ (Class|Actor|GetInputAxisKeyValue) _yaw_2)) false false))))))
    (:then_2
      (Variables|Default|SetPreviousX _locationx_2)
      (Variables|Default|SetPreviousY _locationy_2)
      (Transformation|SetActorRotation (Variables|Default|GetStoredPawn) (Math|Rotator|MakeRotator 0.0 0.0 _yaw))
      (Pawn|SetControlRotation (Math|Rotator|MakeRotator _roll (+ _pitch (* (* (- _locationy (Variables|Default|GetPreviousY)) 0.07) 4.0)) (+ _yaw (* (* (- _locationx (Variables|Default|GetPreviousX)) 0.07) 4.0)))))))

(event Input|ActionEvents|InputActionPlaceFood1
  (params (Key :type Key%20Structure))
  (bind _gamemode (Variables|Default|GetGameMode))
  (:Pressed
    (switch int (Math|Random|RandomIntegerinRange 0 4)
      (:0
        (CallFunction|PlaceFood "/Game/Blueprints/Food/Apple.Apple_C"))
      (:1
        (CallFunction|PlaceFood "/Game/Blueprints/Food/Banana.Banana_C"))
      (:2
        (CallFunction|PlaceFood "/Game/Blueprints/Food/Watermelon.Watermelon_C"))
      (:3
        (CallFunction|PlaceFood "/Game/Blueprints/Food/Carrot.Carrot_C"))
      (:4
        (CallFunction|PlaceFood "/Game/Blueprints/Food/Lettuce.Lettuce_C")))
    (Variables|/Game/Blueprints/AIS_GameMode.AIS_GameMode_C|SetScore _gamemode (- (Variables|/Game/Blueprints/AIS_GameMode.AIS_GameMode_C|GetScore _gamemode) 2))))

(event Input|ActionEvents|InputActionPlaceFood2
  (params (Key :type Key%20Structure))
  (bind _gamemode (Variables|Default|GetGameMode))
  (:Pressed
    (switch int (Math|Random|RandomIntegerinRange 0 1)
      (:0
        (CallFunction|PlaceFood "/Game/Blueprints/Food/Bread.Bread_C"))
      (:1
        (CallFunction|PlaceFood "/Game/Blueprints/Food/Potato.Potato_C")))
    (Variables|/Game/Blueprints/AIS_GameMode.AIS_GameMode_C|SetScore _gamemode (- (Variables|/Game/Blueprints/AIS_GameMode.AIS_GameMode_C|GetScore _gamemode) 2))))

(event Input|ActionEvents|InputActionPlaceFood7
  (params (Key :type Key%20Structure))
  (bind _gamemode (Variables|Default|GetGameMode))
  (:Pressed
    (switch int (Math|Random|RandomIntegerinRange 0 9)
      (:0
        (CallFunction|PlaceFood "/Game/Blueprints/Food/Fish.Fish_C" :!label _label))
      (:1
        (goto _label))
      (:2
        (goto _label))
      (:3
        (goto _label))
      (:4
        (CallFunction|PlaceFood "/Game/Blueprints/Food/Meat.Meat_C" :!label _label_2))
      (:5
        (goto _label_2))
      (:6
        (goto _label_2))
      (:7
        (goto _label_2))
      (:8
        (goto _label_2))
      (:9
        (goto _label_2)))
    (Variables|/Game/Blueprints/AIS_GameMode.AIS_GameMode_C|SetScore _gamemode (- (Variables|/Game/Blueprints/AIS_GameMode.AIS_GameMode_C|GetScore _gamemode) 2))))

(event Input|ActionEvents|InputActionPlaceFood3
  (params (Key :type Key%20Structure))
  (bind _gamemode (Variables|Default|GetGameMode))
  (:Pressed
    (switch int (Math|Random|RandomIntegerinRange 0 1)
      (:0
        (CallFunction|PlaceFood "/Game/Blueprints/Food/Cheese.Cheese_C"))
      (:1
        (CallFunction|PlaceFood "/Game/Blueprints/Food/Milk.Milk_C")))
    (Variables|/Game/Blueprints/AIS_GameMode.AIS_GameMode_C|SetScore _gamemode (- (Variables|/Game/Blueprints/AIS_GameMode.AIS_GameMode_C|GetScore _gamemode) 2))))

(event Input|ActionEvents|InputActionPlaceFood4
  (params (Key :type Key%20Structure))
  (bind _gamemode (Variables|Default|GetGameMode))
  (:Pressed
    (CallFunction|PlaceFood "/Game/Blueprints/Food/Egg.Egg_C")
    (Variables|/Game/Blueprints/AIS_GameMode.AIS_GameMode_C|SetScore _gamemode (- (Variables|/Game/Blueprints/AIS_GameMode.AIS_GameMode_C|GetScore _gamemode) 2))))

(event Input|ActionEvents|InputActionPlaceFood5
  (params (Key :type Key%20Structure))
  (bind _gamemode (Variables|Default|GetGameMode))
  (:Pressed
    (CallFunction|PlaceFood "/Game/Blueprints/Food/Donut.Donut_C")
    (Variables|/Game/Blueprints/AIS_GameMode.AIS_GameMode_C|SetScore _gamemode (- (Variables|/Game/Blueprints/AIS_GameMode.AIS_GameMode_C|GetScore _gamemode) 2))))

(event Input|ActionEvents|InputActionPlaceFood6
  (params (Key :type Key%20Structure))
  (bind _gamemode (Variables|Default|GetGameMode))
  (:Pressed
    (CallFunction|PlaceFood "/Game/Blueprints/Food/Rice_And_Beans.Rice_And_Beans_C")
    (Variables|/Game/Blueprints/AIS_GameMode.AIS_GameMode_C|SetScore _gamemode (- (Variables|/Game/Blueprints/AIS_GameMode.AIS_GameMode_C|GetScore _gamemode) 2))))

(event Input|ActionEvents|InputActionSunLight
  (params (Key :type Key%20Structure))
  (bind _gamemode (Variables|Default|GetGameMode))
  (:Pressed
    (CallFunction|PlaceObject "/Game/Blueprints/SunLight.SunLight_C")
    (Variables|/Game/Blueprints/AIS_GameMode.AIS_GameMode_C|SetScore _gamemode (- (Variables|/Game/Blueprints/AIS_GameMode.AIS_GameMode_C|GetScore _gamemode) 2))))

(event Input|ActionEvents|InputActionPause
  (params (Key :type Key%20Structure))
  ;[1 1 1] Pause the game
  (:Pressed
    (CallFunction|PauseGame)))

(event Input|ActionEvents|InputActionPlaceFood8
  (params (Key :type Key%20Structure))
  (bind _gamemode (Variables|Default|GetGameMode))
  (:Pressed
    (CallFunction|PlaceFood "/Game/Blueprints/Food/Water.Water_C")
    (Variables|/Game/Blueprints/AIS_GameMode.AIS_GameMode_C|SetScore _gamemode (- (Variables|/Game/Blueprints/AIS_GameMode.AIS_GameMode_C|GetScore _gamemode) 2))))

(event Input|AxisEvents|InputAxisMoveForward
  (params (AxisValue :type Float%20%28single-precision%29))
  (bind _returnvalue (Pawn|GetControlRotation :!class /Script/Engine.Controller))
  (Transformation|AddActorLocalOffset (Variables|Default|GetStoredPawn) (* (* (+ (* (Math|Vector|GetForwardVector _returnvalue) AxisValue) (* (Math|Vector|GetRightVector _returnvalue) (stale Input|AxisEvents|InputAxisMoveRight AxisValue))) (Variables|Default|GetMovementRate)) "1.000000,1.000000,0.000000") true false)
  (Transformation|SetWorldRotation (Variables|/Game/Blueprints/AIS_PlayerPawn.AIS_PlayerPawn_C|GetControllerArrow (Variables|Default|GetStoredPawn)) (Pawn|GetControlRotation :!class /Script/Engine.Controller) false false))

(event Input|AxisEvents|InputAxisMoveRight
  (params (AxisValue :type Float%20%28single-precision%29))
  (bind _returnvalue (Pawn|GetControlRotation :!class /Script/Engine.Controller))
  (Transformation|AddActorLocalOffset (Variables|Default|GetStoredPawn) (* (* (+ (* (Math|Vector|GetForwardVector _returnvalue) (stale Input|AxisEvents|InputAxisMoveForward AxisValue)) (* (Math|Vector|GetRightVector _returnvalue) AxisValue)) (Variables|Default|GetMovementRate)) "1.000000,1.000000,0.000000") true false)
  (Transformation|SetWorldRotation (Variables|/Game/Blueprints/AIS_PlayerPawn.AIS_PlayerPawn_C|GetControllerArrow (Variables|Default|GetStoredPawn)) (Pawn|GetControlRotation :!class /Script/Engine.Controller) false false))

(event Input|MouseEvents|LeftMouseButton
  (params (Key :type Key%20Structure))
  (bind _hitresult (Game|Player|GetHitResultUnderCursorbyChannel "TraceTypeQuery2" true))
  (bind _storedpawn (Variables|Default|GetStoredPawn))
  (bind (_bblockinghit _binitialoverlap _time _distance _location _impactpoint _normal _impactnormal _physmat _hitactor) (Collision|BreakHitResult _hitresult))
  (bind _hud (Variables|/Game/Blueprints/AIS_PlayerPawn.AIS_PlayerPawn_C|GetHUD _storedpawn))
  (bind _returnvalue (UserInterface|GetUserWidgetObject _hud))
  (bind _asstat_block (Utilities|Casting|CastToStatBlock _returnvalue))
  (:Pressed
    (if (Utilities|DoesObjectImplementInterface _hitactor "/Game/Interfaces/IsUsable.IsUsable_C")
      (Development|PrintString (Utilities|GetDisplayName _hitactor))
      (Utilities|IsValid (Variables|Default|GetSelectedThing)
        (:Is%20Valid
          (Class|IsUsable|Deselected(Message) (Variables|Default|GetSelectedThing)))
        (:Is%20Not%20Valid
          _))
      (bind _output_get (Variables|Default|SetSelectedThing _hitactor))
      (Class|IsUsable|Selected(Message) _output_get)
      (Variables|/Game/UI/StatBlock.StatBlock_C|SetOwningPawn _asstat_block (.AsAIS%20Character (Utilities|Casting|CastToAIS_Character _output_get)))
      (Default|UpdateHUD _asstat_block)
      (Widget|SetVisibility _asstat_block "Visible")
      (elif (> (Class|PlayerController|GetInputKeyTimeDown Key) 0.0)
        (Timeline|SpawnHold PlayFromStart))))
  (:Released
    (Timeline|SpawnHold Stop)))

(event Input|MouseEvents|RightMouseButton
  (params (Key :type Key%20Structure))
  (bind _storedpawn (Variables|Default|GetStoredPawn))
  (bind _springarm (Variables|/Game/Blueprints/AIS_PlayerPawn.AIS_PlayerPawn_C|GetSpringArm _storedpawn))
  (bind _returnvalue (Transformation|GetWorldRotation _springarm))
  (bind (_roll _pitch _yaw) (Math|Rotator|BreakRotator _returnvalue))
  (:Pressed
    (Variables|Default|SetbRightClick true)
    (Utilities|FlowControl|Gate true) ; enters at Open
  )
  (:Released
    (if (not (Variables|Default|GetbRightClick))
      _
      (else
        (CallFunction|RightClickAction)))
    (Variables|Default|SetRightClickHoldCounter 0.0)
    (Utilities|FlowControl|Gate true) ; enters at Close
  ))

(fn ConstructionScript)

(fn PlaceFood
  (params (FoodType :type Actor%20Class%20Reference))
  (bind _hitresult (Game|Player|GetHitResultUnderCursorbyChannel "TraceTypeQuery2" true))
  (bind _location (Collision|BreakHitResult _hitresult))
  (bind (_x _y _z) (Math|Vector|BreakVector _location))
  (bind _returnvalue (Game|SpawnActorfromClass FoodType (Math|Conversions|ToTransform(Vector) (Math|Vector|MakeVector _x _y (+ _z 5e+01))) "Undefined" 0 0))
  (bind _asgood_food (Utilities|Casting|CastToGoodFood _returnvalue))
  (Class|PrimitiveComponent|SetPhysicsAngularVelocityinDegrees (Variables|/Game/Blueprints/Food/GoodFood.GoodFood_C|GetFoodMesh _asgood_food) (* (Math|Random|RandomUnitVector) 1e+02) false "None"))

(fn PlaceObject
  (params (Sunlight :type Actor%20Class%20Reference))
  (bind _hitresult (Game|Player|GetHitResultUnderCursorbyChannel "TraceTypeQuery2" true))
  (bind _location (Collision|BreakHitResult _hitresult))
  (bind (_x _y _z) (Math|Vector|BreakVector _location))
  (Game|SpawnActorfromClass Sunlight (Math|Transform|MakeTransform (Math|Vector|MakeVector _x _y (+ _z 5.0)) "0, 0, 0" "0.500000,0.500000,0.500000") "Undefined" 0 0))

(fn PauseGame
  (Utilities|FlowControl|Sequence
    (:then_0
      (bind _asais_game_mode (Utilities|Casting|CastToAIS_GameMode (Game|GetGameMode)))
      (Widget|SetVisibility (Variables|/Game/Blueprints/AIS_GameMode.AIS_GameMode_C|GetScore_Widget _asais_game_mode) "Hidden"))
    (:then_1
      (Game|SetGamePaused true)
      (Utilities|IsValid (Variables|Default|GetPause%20Menu)
        (:Is%20Valid
          (Widget|SetVisibility (Variables|Default|GetPause%20Menu) "Visible")
          (Input|SetInputModeGameandUI (Game|GetPlayerController 0) (Variables|Default|GetPause%20Menu) "DoNotLock" false)
          (Variables|/Script/Engine.PlayerController|SetbShowMouseCursor (Game|GetPlayerController 0) true))
        (:Is%20Not%20Valid
          (bind _returnvalue (UserInterface|CreateWidget "/Game/UI/Pause_Menu.Pause_Menu_C" (Game|GetPlayerController 0)))
          (bind _output_get (Variables|Default|SetPause%20Menu _returnvalue))
          (UserInterface|Viewport|AddtoViewport _output_get 0))))))

(fn UnpauseGame
  (bind _returnvalue (Game|GetPlayerController 0))
  (Game|SetGamePaused false)
  (Widget|SetVisibility (Variables|Default|GetPause%20Menu) "Hidden")
  (Input|SetInputModeGameandUI _returnvalue 0 "LockAlways" false)
  (Variables|/Script/Engine.PlayerController|SetbShowMouseCursor _returnvalue true)
  (bind _asais_game_mode (Utilities|Casting|CastToAIS_GameMode (Game|GetGameMode)))
  (Widget|SetVisibility (Variables|/Game/Blueprints/AIS_GameMode.AIS_GameMode_C|GetScore_Widget _asais_game_mode) "Visible"))